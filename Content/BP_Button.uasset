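; Button actor with an animated press and an overlap box that opens a gate while BP_Player is inside and closes it on exit.
; BeginPlay caches the resting transform and a Y-offset pressed one, then calls Button Animation, which lerps between them using press and reversed-release timelines.
; A BP_Turtle spawn hangs off the animation's Out pin, which is never reached, and the gate has no visible link to the animation.
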(event `self.ReceiveBeginPlay`
  (bind (_returnvalue_location _returnvalue_rotation _returnvalue_scale) (`KismetMathLibrary.BreakTransform` (`SceneComponent.GetRelativeTransform` (`self.Button`))))
  (set `self.Out position` (`KismetMathLibrary.MakeTransform` _returnvalue_location _returnvalue_rotation _returnvalue_scale))
  (set `self.In position` (`KismetMathLibrary.MakeTransform` (- _returnvalue_location (0.0 10.0 0.0)) _returnvalue_rotation _returnvalue_scale))
  (bind (_direction _newtrack_0) (`Timeline|Button In`)
    (:`Update`
      (`SceneComponent.K2_SetRelativeTransform` (`self.Button`) (`KismetMathLibrary.TLerp` (`self.Out position`) (`self.In position`) _newtrack_0) false false))
    (:`Finished`
      (bind (_direction_2 _newtrack_0_2) (`Timeline|Button out` :!via `ReverseFromEnd`)
        (:`Update`
          (`SceneComponent.K2_SetRelativeTransform` (`self.Button`) (`KismetMathLibrary.TLerp` (`self.Out position`) (`self.In position`) _newtrack_0_2) false false))))))

(event `self.Box.OnComponentBeginOverlap`
  (params (OverlappedComponent :type "PrimitiveComponent Object Reference") (OtherActor :type "Actor Object Reference") (OtherComp :type "PrimitiveComponent Object Reference") (OtherBodyIndex :type Integer) (bFromSweep :type Boolean) (SweepResult :type "HitResult Structure (by ref)"))
  ;[1 1 1] Push button
  (cast `/Game/BP_Player` OtherActor)
  (`/Engine/EditorBlueprintResources/StandardMacros.Gate` true :!via `Open` :!label _label))

(event `self.Box.OnComponentEndOverlap`
  (params (OverlappedComponent :type "PrimitiveComponent Object Reference") (OtherActor :type "Actor Object Reference") (OtherComp :type "PrimitiveComponent Object Reference") (OtherBodyIndex :type Integer))
  ;[1 1 1] Push button
  (cast `/Game/BP_Player` OtherActor)
  (goto _label :!via `Close`))

(fn `UserConstructionScript`)